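; BP_Granade is a timed grenade actor that explodes when its countdown runs out.
; Tick counts TimeToDetonate down to zero, then spawns a particle system and sound at Sphere1's location.
; It calls KillInRange on the Helpline Detroit game mode with KillRange, then fires an impulse from a runtime-added radial force component and destroys itself.
; The 0.2-second Delay sits on its own sequence branch, so it holds back neither impulse nor destruction.
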(event `self.ReceiveTick`
  (params (DeltaSeconds :type "Float (single-precision)"))
  (bind _returnvalue (`SceneComponent.K2_GetComponentLocation` (`self.Sphere1`)))
  (bind _output_get (set `self.TimeToDetonate` (- (`self.TimeToDetonate`) DeltaSeconds)))
  (if (<= _output_get 0.0)
    (`|ExecutionSequence`
      (:`then_0`
        (`NiagaraFunctionLibrary.SpawnSystemAtLocation` "/Game/HelplineDetroit/ASSETS/Explosion.Explosion" _returnvalue (struct) (1.0 1.0 1.0) true true "AutoRelease"))
      (:`then_1`
        (`GameplayStatics.PlaySoundAtLocation` "/Game/HelplineDetroit/ASSETS/SFX_Explosion.SFX_Explosion" _returnvalue (struct) 1.0 1.0 0.0 null null null null))
      (:`then_2`
        (bind _asbp_past_and_future_game_mode (cast `/Game/HelplineDetroit/BP_HelplineDetroit_GameMode` (`GameplayStatics.GetGameMode`)))
        (`/Game/HelplineDetroit/BP_HelplineDetroit_GameMode.Kill In Range` _asbp_past_and_future_game_mode _returnvalue (`self.Kill Range`)))
      (:`then_3`
        (`KismetSystemLibrary.Delay` 0.2))
      (:`then_4`
        (bind _returnvalue_2 (`AddComponent|NODE_AddRadialForceComponent-1` :`bManualAttachment` true :`RelativeTransform` (`KismetMathLibrary.MakeTransform` (`SceneComponent.RelativeLocation` (`self.Sphere1`)))))
        (`RadialForceComponent.FireImpulse` _returnvalue_2))
      (:`then_5`
        (`self.K2_DestroyActor`)))))

(fn `UserConstructionScript`)