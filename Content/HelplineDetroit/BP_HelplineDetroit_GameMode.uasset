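; Game mode for HelplineDetroit that handles session startup and offers an area damage event against enemies.
; On BeginPlay it loads or creates the save object, hides the mouse cursor and prints a long-lasting controls hint.
; KillInRange sphere-overlaps enemy pawns around a given position and applies a fixed point of damage to each.
; The SaveGame event is an empty stub, so saving only happens when a new save is created.
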(event `self.ReceiveBeginPlay`
  (`|ExecutionSequence`
    (:`then_0`
      (bind _returnvalue (`GameplayStatics.LoadGameFromSlot` "SaveData"))
      (`/Engine/EditorBlueprintResources/StandardMacros.IsValid` _returnvalue
        (:`Is Valid`
          (bind _asbp_save_game (cast `/Game/HelplineDetroit/BP_SaveGame` _returnvalue))
          (set `self.save data` _asbp_save_game))
        (:`Is Not Valid`
          (bind _returnvalue_2 (`GameplayStatics.CreateSaveGameObject` "/Game/HelplineDetroit/BP_SaveGame.BP_SaveGame_C"))
          (bind _output_get (set `self.save data` _returnvalue_2))
          (`GameplayStatics.SaveGameToSlot` _output_get "SaveData"))))
    (:`then_1`
      (set `PlayerController.bShowMouseCursor` false (`GameplayStatics.GetPlayerController` 0)))
    (:`then_2`
      (`KismetSystemLibrary.PrintText` (`KismetTextLibrary.Conv_StringToText` (`KismetStringLibrary.JoinStringArray` (`|MakeArray` "WSAD - Move" "Mouse - Aim" "Mouse Scroll - Change weapon" "Esc - Return to menu") " \n")) true true (struct :`G` 0.66 :`B` 1.0 :`A` 1.0) 1000.0))))

(event `Kill In Range`
  (params (`World Position` :type "Vector Structure") (Range :type "Float (double-precision)"))
  (bind _outactors (`KismetSystemLibrary.SphereOverlapActors` `World Position` Range (`|MakeArray` "ObjectTypeQuery3" :!type "EObjectTypeQuery Enum") "/Game/HelplineDetroit/BP_Enemy.BP_Enemy_C"))
  (for _array_element _outactors
    (`GameplayStatics.ApplyDamage` _array_element 1.0)))

(event `Event Save Game`)

(fn `UserConstructionScript`)