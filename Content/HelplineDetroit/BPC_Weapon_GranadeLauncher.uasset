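; BPC_Weapon_GranadeLauncher is a grenade launcher weapon component that fires a physical grenade when its Shoot event runs.
; Shoot plays a thump sound in 2D and spawns a BP_Granade at the component's world location and rotation, regardless of collisions.
; It then launches the grenade with a single large AddForce on its Sphere1 body along the grenade mesh's forward vector.
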(event `self.Shoot`
  (`GameplayStatics.PlaySound2D` "/Game/HelplineDetroit/ASSETS/SFX_Thump.SFX_Thump" 1.0 1.0 0.0 null null)
  (bind _returnvalue (`|SpawnActorFromClass` "/Game/HelplineDetroit/BP_Granade.BP_Granade_C" (`KismetMathLibrary.MakeTransform` (`self.K2_GetComponentLocation`) (`self.K2_GetComponentRotation`)) "AlwaysSpawn" "MultiplyWithRoot" null null))
  (`self.AddForce` (`/Game/HelplineDetroit/BP_Granade.Sphere1` _returnvalue) (* (`self.GetForwardVector` (`/Game/HelplineDetroit/BP_Granade.granade` _returnvalue)) 500000.0) "None" false))