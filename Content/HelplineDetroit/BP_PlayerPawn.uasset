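; Top-down player pawn for a shooter, with world-axis movement, mouse-cursor aiming and four switchable weapons.
; Each tick it turns its Arrow component's yaw toward the point under the cursor.
; Weapon components share the BPC_Weapon interface for left-click shoot and stop, while the mouse wheel cycles them with negative-safe wrapping, showing only the current one.
; Escape opens the startup map, and a debug print of the slot index remains on switching.
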(event `self.ReceiveBeginPlay`
  (bind _returnvalue (`GameplayStatics.GetPlayerController` 0))
  (`WidgetBlueprintLibrary.SetInputMode_GameOnly` _returnvalue true)
  (`self.EnableInput` _returnvalue)
  (set `self.Weapons` (`|MakeArray` (`self.BPC_Weapon_Handgun`) (`self.BPC_Weapon_Machinegun`) (`self.BPC_Weapon_Shotgun`) (`self.BPC_Weapon_GranadeLauncher1`) :!type "StaticMeshComponent Object Reference"))
  (`self.Switch Weapon` (`self.Current Weapon`)))

(event `self.ReceiveTick`
  (params (DeltaSeconds :type "Float (single-precision)"))
  (bind (_returnvalue_roll _returnvalue_pitch _returnvalue_yaw) (`KismetMathLibrary.BreakRotator` (`KismetMathLibrary.FindLookAtRotation` (`self.K2_GetActorLocation`) (`.Location` (`GameplayStatics.BreakHitResult` (`PlayerController.GetHitResultUnderCursorByChannel` (`GameplayStatics.GetPlayerController` 0) "TraceTypeQuery1" false))))))
  (`SceneComponent.K2_SetWorldRotation` (`self.Arrow`) (`KismetMathLibrary.MakeRotator` 0.0 0.0 _returnvalue_yaw) true false))

(event `Key|Escape`
  (params (Key :type "Key Structure"))
  (:`Pressed`
    (`GameplayStatics.OpenLevelBySoftObjectPtr` "/Game/Maps/StartupMap.StartupMap")))

(event `InputAxis|ForwardAxis`
  (params (AxisValue :type "Float (single-precision)"))
  (`self.AddMovementInput` (1.0 0.0 0.0) AxisValue))

(event `InputAxis|RightAxis`
  (params (AxisValue :type "Float (single-precision)"))
  (`self.AddMovementInput` (0.0 1.0 0.0) AxisValue))

(event `Key|LeftMouseButton`
  (params (Key :type "Key Structure"))
  (bind _output (`|GetArrayItem` (`self.Weapons`) (`self.Current Weapon`)))
  (:`Pressed`
    (bind _asbpc_weapon (cast `/Game/HelplineDetroit/BPC_Weapon` _output))
    (`/Game/HelplineDetroit/BPC_Weapon.Shoot` _asbpc_weapon))
  (:`Released`
    (bind _asbpc_weapon_2 (cast `/Game/HelplineDetroit/BPC_Weapon` _output))
    (`/Game/HelplineDetroit/BPC_Weapon.Stop Shooting` _asbpc_weapon_2)))

(event `InputAxisKey|MouseWheelAxis`
  (params (AxisValue :type "Float (single-precision)"))
  (bind _returnvalue (`self.Wrap Integer` (+ (`self.Current Weapon`) (`KismetMathLibrary.Round` AxisValue)) (`KismetArrayLibrary.Array_Length` (`self.Weapons`))))
  (if (!= AxisValue 0.0)
    (`KismetSystemLibrary.PrintString` (`KismetStringLibrary.Conv_IntToString` _returnvalue))
    (bind _output_get (set `self.Current Weapon` _returnvalue))
    (`self.Switch Weapon` _output_get)))

(fn `Switch Weapon`
  (params (`Current Weapon Slot` :type Integer))
  (for (_array_element _array_index) (`self.Weapons`)
    (if (== _array_index `Current Weapon Slot`)
      (`SceneComponent.SetHiddenInGame` _array_element false true)
      (else
        (`SceneComponent.SetHiddenInGame` _array_element true true)))))

(fn `UserConstructionScript`)

(fn `Wrap Integer`
  (params (value :type Integer) (`max value` :type Integer))
  (returns (ReturnValue :type Integer))
  (bind _returnvalue (mod value `max value`))
  (if (< _returnvalue 0)
    (return (+ `max value` _returnvalue))
    (else
      (return _returnvalue))))