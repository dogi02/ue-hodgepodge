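; BPC_Weapon_Handgun is a handgun component that fires a hitscan shot when its Shoot event runs.
; Shoot plays a 2D gunshot sound and line-traces a short fixed range along the component's forward vector on the Visibility channel, drawing a debug line.
; It applies flat damage to the hit actor and, on physics-simulating components, adds HitForce against the hit normal at the impact point.
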(event `self.Shoot`
  (bind _returnvalue (`self.K2_GetComponentLocation`))
  (bind _returnvalue_2 (+ _returnvalue (* (`self.GetForwardVector`) (`KismetMathLibrary.Conv_DoubleToVector` 1000.0))))
  (`GameplayStatics.PlaySound2D` "/Game/HelplineDetroit/ASSETS/SFX_Gunshot.SFX_Gunshot" 1.0 1.0 0.0 null null)
  (`KismetSystemLibrary.DrawDebugLine` _returnvalue _returnvalue_2 (struct :`R` 1.0 :`B` 0.075413 :`A` 1.0) 1.0 1.0)
  (bind _outhit (`KismetSystemLibrary.LineTraceSingle` _returnvalue _returnvalue_2 "TraceTypeQuery1"))
  (`GameplayStatics.ApplyDamage` (`.HitActor` (`GameplayStatics.BreakHitResult` _outhit)) 1.0)
  (if (`self.IsSimulatingPhysics` (`.HitComponent` (`GameplayStatics.BreakHitResult` _outhit)) "None")
    (`self.AddForceAtLocation` (`.HitComponent` (`GameplayStatics.BreakHitResult` _outhit)) (* (`.Normal` (`GameplayStatics.BreakHitResult` _outhit)) (`self.hitForce`) -1.0) (`.ImpactPoint` (`GameplayStatics.BreakHitResult` _outhit)) "None")))