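; Shotgun weapon component whose Shoot event fires a flat horizontal fan of short hitscan pellets at one-degree steps around its forward vector.
; Two sequenced loops cover either side of the fan, the second including the centre, each playing its own sound per pellet.
; Every pellet draws a debug line, traces on Visibility, applies damage and pushes physics-simulating components against the hit normal using HitForce.
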(event `self.Shoot`
  (bind _returnvalue (`self.K2_GetComponentLocation`))
  (bind _returnvalue_2 (`self.K2_GetComponentLocation`))
  (`|ExecutionSequence`
    (:`then_0`
      (for _index (range 1 4)
        (`GameplayStatics.PlaySound2D` "/Game/HelplineDetroit/ASSETS/SFX_Thump.SFX_Thump" 1.0 1.0 0.0 null null)
        (bind _returnvalue_3 (+ _returnvalue (* (`KismetMathLibrary.RotateAngleAxis` (`self.GetForwardVector`) (`KismetMathLibrary.Conv_IntToDouble` (* _index -1)) (0.0 0.0 1.0)) (`KismetMathLibrary.Conv_DoubleToVector` 1000.0))))
        (`KismetSystemLibrary.DrawDebugLine` _returnvalue _returnvalue_3 (struct :`R` 1.0 :`B` 0.075413 :`A` 1.0) 1.0 1.0)
        (bind _outhit (`KismetSystemLibrary.LineTraceSingle` _returnvalue _returnvalue_3 "TraceTypeQuery1"))
        (`GameplayStatics.ApplyDamage` (`.HitActor` (`GameplayStatics.BreakHitResult` _outhit)) 1.0)
        (if (`self.IsSimulatingPhysics` (`.HitComponent` (`GameplayStatics.BreakHitResult` _outhit)) "None")
          (`self.AddForceAtLocation` (`.HitComponent` (`GameplayStatics.BreakHitResult` _outhit)) (* (`.Normal` (`GameplayStatics.BreakHitResult` _outhit)) (`self.hitForce`) -1.0) (`.ImpactPoint` (`GameplayStatics.BreakHitResult` _outhit)) "None"))))
    (:`then_1`
      (for _index_2 (range 4)
        (`GameplayStatics.PlaySound2D` "/Game/HelplineDetroit/ASSETS/SFX_Gunshot.SFX_Gunshot" 1.0 1.0 0.0 null null)
        (bind _returnvalue_4 (+ _returnvalue_2 (* (`KismetMathLibrary.RotateAngleAxis` (`self.GetForwardVector`) (`KismetMathLibrary.Conv_IntToDouble` _index_2) (0.0 0.0 1.0)) (`KismetMathLibrary.Conv_DoubleToVector` 1000.0))))
        (`KismetSystemLibrary.DrawDebugLine` _returnvalue_2 _returnvalue_4 (struct :`R` 1.0 :`B` 0.075413 :`A` 1.0) 1.0 1.0)
        (bind _outhit_2 (`KismetSystemLibrary.LineTraceSingle` _returnvalue_2 _returnvalue_4 "TraceTypeQuery1"))
        (`GameplayStatics.ApplyDamage` (`.HitActor` (`GameplayStatics.BreakHitResult` _outhit_2)) 1.0)
        (if (`self.IsSimulatingPhysics` (`.HitComponent` (`GameplayStatics.BreakHitResult` _outhit_2)) "None")
          (`self.AddForceAtLocation` (`.HitComponent` (`GameplayStatics.BreakHitResult` _outhit_2)) (* (`.Normal` (`GameplayStatics.BreakHitResult` _outhit_2)) (`self.hitForce`) -1.0) (`.ImpactPoint` (`GameplayStatics.BreakHitResult` _outhit_2)) "None"))))))