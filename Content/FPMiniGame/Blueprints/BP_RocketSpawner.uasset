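; BP_RocketSpawner is a moving launcher in the FPMiniGame that periodically fires homing rockets at targets.
; A looping timer spawns a BP_Rocket at the Sphere's position every ShootCooldown and homes it on a random Target entry's RocketTarget component.
; A Timeline ping-pongs the Sphere between StartPos and EndPos, with its play rate scaled so each pass takes MoveTime.
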(event `self.ReceiveBeginPlay`
  (bind _timeline (`self.Timeline`))
  (`KismetSystemLibrary.K2_SetTimerDelegate` (delegate `LaunchRocket`) (`self.ShootCooldown`) true)
  (`TimelineComponent.SetPlayRate` _timeline (/ (`TimelineComponent.GetTimelineLength` _timeline) (`self.MoveTime`)))
  (`self.Move`))

(event `LaunchRocket`
  (bind _target (`self.Target`))
  (bind _returnvalue (`|SpawnActorFromClass` "/Game/FPMiniGame/Blueprints/BP_Rocket.BP_Rocket_C" (`KismetMathLibrary.MakeTransform` (`SceneComponent.K2_GetComponentLocation` (`self.Sphere`))) "Undefined" "MultiplyWithRoot" null null))
  (set `ProjectileMovementComponent.HomingTargetComponent` (`/Game/FPMiniGame/Blueprints/BP_Base.RocketTarget` (`|GetArrayItem` _target (`KismetMathLibrary.RandomIntegerInRange` 0 (- (`KismetArrayLibrary.Array_Length` _target) 1)))) (`/Game/FPMiniGame/Blueprints/BP_Rocket.ProjectileMovement` _returnvalue)))

(event `Move`
  (bind _timeline (`self.Timeline`))
  (bind (_direction _alpha) (`Timeline|Timeline` :!via `PlayFromStart`)
    (:`Update`
      (`SceneComponent.K2_SetRelativeLocation` (`self.Sphere`) (`KismetMathLibrary.VLerp` (`self.StartPos`) (`self.EndPos`) _alpha) false false))
    (:`Finished`
      (if (`|EnumEquality` _direction "Forward")
        (`TimelineComponent.ReverseFromEnd` _timeline)
        (else
          (`TimelineComponent.PlayFromStart` _timeline))))))

(fn `UserConstructionScript`)