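; BP_Player is the player Blueprint for Rocket Defence, where clicking destroys incoming rockets before every base is lost.
; Left click runs a sphere trace at the cursor's hit point, destroying each BP_Rocket found and spawning a burst effect.
; A looping one-second timer updates the W_RocketDefence countdown and polls the base list.
; Losing all bases shows the lose panel; outlasting the countdown shows the win panel, and either pauses the timer.
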(event `StartTimer`
  ;[1 1 1] Timer
  (bind _returnvalue (`KismetSystemLibrary.K2_SetTimerDelegate` (delegate `Timer`) 1.0 true))
  (set `self.TimerHandle` _returnvalue))

(event `self.ReceiveBeginPlay`
  ;[1 1 1] Initial Setup
  (set `PlayerController.bShowMouseCursor` true (`GameplayStatics.GetPlayerController` 0))
  (`self.StartTimer`)
  (bind _returnvalue (`|CreateWidget` "/Game/RocketDefence/W_RocketDefence.W_RocketDefence_C" (`GameplayStatics.GetPlayerController` 0)))
  (bind _output_get (set `self.PlayerWidget` _returnvalue))
  (`UserWidget.AddToViewport` _output_get 0))

(event `Timer`
  ;[1 1 1] Timer
  (bind _result (`/Engine/EditorBlueprintResources/StandardMacros.IncrementInt` (`self.Time`))
    (:`  `
      (bind _returnvalue (- (`self.GameTimeLength`) _result))
      (set `self.TimeLeft` _returnvalue)
      (`self.CheckWinLoseCondition`)
      (set `TextBlock.Text` (`KismetTextLibrary.Conv_IntToText` _returnvalue) (`/Game/RocketDefence/W_RocketDefence.Timer` (`self.PlayerWidget`))))))

(event `Key|LeftMouseButton`
  (params (Key :type "Key Structure"))
  (bind (_bblockinghit _binitialoverlap _time _distance _location) (`GameplayStatics.BreakHitResult` (`PlayerController.GetHitResultUnderCursorByChannel` (`GameplayStatics.GetPlayerController` 0) "TraceTypeQuery1" true)))
  ;[1 1 1] Destroying Rockets with LMB
  (:`Pressed`
    (bind _outhits (`KismetSystemLibrary.SphereTraceMulti` _location _location 50.0 "TraceTypeQuery1"))
    (for _array_element _outhits
      (bind _asbp_rocket (cast `/Game/RocketDefence/Blueprints/BP_Rocket` (`.HitActor` (`GameplayStatics.BreakHitResult` _array_element))))
      (`/Game/RocketDefence/Blueprints/BP_Rocket.DestroyRocket` _asbp_rocket)
      (`NiagaraFunctionLibrary.SpawnSystemAtLocation` "/Niagara/DefaultAssets/Templates/Systems/RadialBurst.RadialBurst" _location (struct :`Pitch` -90.0)))))

(event `PauseTimer`
  ;[1 1 1] Timer
  (`KismetSystemLibrary.K2_PauseTimerHandle` (`self.TimerHandle`)))

(event `ResumeTimer`
  ;[1 1 1] Timer
  (`KismetSystemLibrary.K2_UnPauseTimerHandle` (`self.TimerHandle`)))

(event `CheckWinLoseCondition`
  (bind _baselist (`self.BaseList`))
  ;[1 1 1] Win/Lose
  (for _array_element (`self.BaseList`)
    (if (`/Game/RocketDefence/Blueprints/BP_Base.Destroyed` _array_element)
      (`KismetArrayLibrary.Array_RemoveItem` _baselist _array_element)
      (if (== (`KismetArrayLibrary.Array_Length` _baselist) 0)
        (`self.Lose`))))
  (if (== (`self.TimeLeft`) 0)
    (if (not (== (`KismetArrayLibrary.Array_Length` (`self.BaseList`)) 0))
      (`self.Win`))))

(event `Lose`
  ;[1 1 1] Win/Lose
  (if (not (== (`self.TimeLeft`) 0))
    (`self.PauseTimer`)
    (`Widget.SetVisibility` (`/Game/RocketDefence/W_RocketDefence.LosePanel` (`self.PlayerWidget`)) "Visible")))

(event `Win`
  ;[1 1 1] Win/Lose
  (`self.PauseTimer`)
  (`Widget.SetVisibility` (`/Game/RocketDefence/W_RocketDefence.WinPanel` (`self.PlayerWidget`)) "Visible"))

(fn `UserConstructionScript`)