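; BP_RocketSpawner is a rocket launcher for Rocket Defence that slides back and forth while firing homing rockets at targets.
; A looping timer spawns a scaled-down rocket at the Sphere's location and sets its homing component to a random Target entry's RocketTarget.
; A Timeline, rate-scaled to MoveTime, lerps the mesh between StartPos and EndPos, with its Finished output meant to alternate direction for continuous ping-pong movement.
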(event `self.ReceiveBeginPlay`
  (bind _timeline (`self.Timeline`))
  (`KismetSystemLibrary.K2_SetTimerDelegate` (delegate `LaunchRocket`) (`self.ShootCooldown`) true)
  (`TimelineComponent.SetPlayRate` _timeline (/ (`TimelineComponent.GetTimelineLength` _timeline) (`self.MoveTime`)))
  (`self.Move`))

(event `LaunchRocket`
  (bind _returnvalue (`|SpawnActorFromClass` "/Game/RocketDefence/Blueprints/BP_Rocket.BP_Rocket_C" (`KismetMathLibrary.MakeTransform` (`SceneComponent.K2_GetComponentLocation` (`self.Sphere`)) (struct) (0.25 0.25 0.25)) "Undefined" "MultiplyWithRoot" null null))
  (`self.ChooseTarget` _returnvalue))

(event `Move`
  (bind _timeline (`self.Timeline`))
  (bind (_direction _alpha) (`Timeline|Timeline` :!via `PlayFromStart`)
    (:`Update`
      (`SceneComponent.K2_SetRelativeLocation` (`self.StaticMesh`) (`KismetMathLibrary.VLerp` (`self.StartPos`) (`self.EndPos`) _alpha) false false))
    (:`Finished`
      (if (`|EnumEquality` _direction "Forward")
        (`TimelineComponent.ReverseFromEnd` _timeline)
        (else
          (`TimelineComponent.PlayFromStart` _timeline))))))

(fn `ChooseTarget`
  (params (RocketActor :type "/Game/RocketDefence/Blueprints/BP_Rocket Object Reference"))
  (bind _target (`self.Target`))
  (set `ProjectileMovementComponent.HomingTargetComponent` (`/Game/RocketDefence/Blueprints/BP_Base.RocketTarget` (`|GetArrayItem` _target (`KismetMathLibrary.RandomIntegerInRange` 0 (- (`KismetArrayLibrary.Array_Length` _target) 1)))) (`/Game/RocketDefence/Blueprints/BP_Rocket.ProjectileMovement` RocketActor)))

(fn `UserConstructionScript`)