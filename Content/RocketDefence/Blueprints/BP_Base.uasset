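; BP_Base is a base in the Rocket Defence game that takes damage from incoming rockets.
; When a BP_Rocket overlaps its box, the base runs Hit and then tells the rocket to destroy itself.
; Each hit spawns a Niagara explosion at the mesh and removes one hit point.
; At zero HP it sets a one-time Destroyed flag and swaps the mesh material, leaving the actor in place.
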(event `DestoryBase`
  (if (not (`self.Destroyed`))
    (set `self.Destroyed` true)
    (`PrimitiveComponent.SetMaterial` (`self.Mesh`) 0 "/Game/RocketDefence/Materials/M_Color.M_Color")))

(event `Hit`
  (`NiagaraFunctionLibrary.SpawnSystemAtLocation` "/Game/RocketDefence/Niagara_Explosion.Niagara_Explosion" (`SceneComponent.K2_GetComponentLocation` (`self.Mesh`)) (struct :`Pitch` -90.0))
  (bind _output_get (set `self.CurrentHP` (- (`self.CurrentHP`) 1)))
  (if (<= _output_get 0)
    (`self.DestoryBase`)))

(event `self.Box.OnComponentBeginOverlap`
  (params (OverlappedComponent :type "PrimitiveComponent Object Reference") (OtherActor :type "Actor Object Reference") (OtherComp :type "PrimitiveComponent Object Reference") (OtherBodyIndex :type Integer) (bFromSweep :type Boolean) (SweepResult :type "HitResult Structure (by ref)"))
  (bind _asbp_rocket (cast `/Game/RocketDefence/Blueprints/BP_Rocket` OtherActor))
  (`self.Hit`)
  (`/Game/RocketDefence/Blueprints/BP_Rocket.DestroyRocket` _asbp_rocket))

(fn `UserConstructionScript`)