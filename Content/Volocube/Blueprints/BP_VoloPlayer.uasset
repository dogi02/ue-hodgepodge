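; BP_VoloPlayer is the Volocube player character, kept between two boundary positions on the world X axis.
; Every Tick it compares its location to LocWall1 (upper limit) and LocWall2 (lower limit) and snaps X back to the crossed limit, preserving Y and Z.
; It also prints X velocity as a signed fraction of the movement component's max speed each frame as a debug readout.
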(event `self.ReceiveTick`
  (params (DeltaSeconds :type "Float (single-precision)"))
  (bind (_returnvalue_x _returnvalue_y _returnvalue_z) (`KismetMathLibrary.BreakVector` (`self.K2_GetActorLocation`)))
  (bind _returnvalue_x_2 (`KismetMathLibrary.BreakVector` (`self.GetVelocity`)))
  (if (> _returnvalue_x (`self.LocWall1`))
    (`self.K2_SetActorLocation` (`KismetMathLibrary.MakeVector` (`self.LocWall1`) _returnvalue_y _returnvalue_z))
    (elif (< _returnvalue_x (`self.LocWall2`))
      (`self.K2_SetActorLocation` (`KismetMathLibrary.MakeVector` (`self.LocWall2`) _returnvalue_y _returnvalue_z))))
  (`KismetSystemLibrary.PrintString` (`KismetStringLibrary.Concat_StrStr` "Current Player Speed:" (`KismetStringLibrary.Conv_DoubleToString` (/ _returnvalue_x_2 (`MovementComponent.GetMaxSpeed` (`self.CharacterMovement`))))) true true (struct :`R` 1.0 :`B` 0.03636 :`A` 1.0) 0.0))

(fn `UserConstructionScript`)