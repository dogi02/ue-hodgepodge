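; BP_Ball is a pong-style bouncing ball for Volocube, driven by a FloatingPawnMovement component.
; BeginPlay picks a random diagonal direction in the XY plane, which Tick feeds in as movement input every frame.
; Collision overlaps reflect it by negating one axis: X for BP_Wall, Y for BP_VoloPlayer, each with a debug print.
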(event `self.ReceiveBeginPlay`
  (set `self.BallVelocity` (`KismetMathLibrary.MakeVector` (select `bool` (`KismetMathLibrary.RandomBool`) :`false` -1.0 :`true` 1.0) (select `bool` (`KismetMathLibrary.RandomBool`) :`false` -1.0 :`true` 1.0))))

(event `self.ReceiveTick`
  (params (DeltaSeconds :type "Float (single-precision)"))
  (`PawnMovementComponent.AddInputVector` (`self.FloatingPawnMovement`) (`self.BallVelocity`) false))

(event `self.Collision.OnComponentBeginOverlap`
  (params (OverlappedComponent :type "PrimitiveComponent Object Reference") (OtherActor :type "Actor Object Reference") (OtherComp :type "PrimitiveComponent Object Reference") (OtherBodyIndex :type Integer) (bFromSweep :type Boolean) (SweepResult :type "HitResult Structure (by ref)"))
  (bind (_ballvelocity_x _ballvelocity_y _ballvelocity_z) (`KismetMathLibrary.BreakVector` (`self.BallVelocity`)))
  (bind (_ballvelocity_x_2 _ballvelocity_y_2 _ballvelocity_z_2) (`KismetMathLibrary.BreakVector` (`self.BallVelocity`)))
  (cast `/Game/Volocube/Blueprints/BP_Wall` OtherActor
    (:`then`
      (`KismetSystemLibrary.PrintString` "Wall" true true (struct :`R` 1.0 :`B` 0.471066 :`A` 1.0))
      (set `self.BallVelocity` (`KismetMathLibrary.MakeVector` (* _ballvelocity_x_2 -1.0) _ballvelocity_y_2 _ballvelocity_z_2)))
    (:`CastFailed`
      (cast `/Game/Volocube/Blueprints/BP_VoloPlayer` OtherActor)
      (`KismetSystemLibrary.PrintString` "Player")
      (set `self.BallVelocity` (`KismetMathLibrary.MakeVector` _ballvelocity_x (* _ballvelocity_y -1.0) _ballvelocity_z)))))

(fn `UserConstructionScript`)