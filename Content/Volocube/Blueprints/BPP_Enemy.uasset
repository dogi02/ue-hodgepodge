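; BPP_Enemy is an AI-controlled opponent that chases BP_Ball along the world X axis.
; Each Tick it clamps its X position to fixed bounds, then looks up the ball with GetActorOfClass.
; It adds full movement input toward the ball based only on the sign of the X difference, with no dead zone, and prints that difference for debugging.
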(event `self.ReceiveTick`
  (params (DeltaSeconds :type "Float (single-precision)"))
  (bind (_returnvalue_x _returnvalue_y _returnvalue_z) (`KismetMathLibrary.BreakVector` (`self.K2_GetActorLocation`)))
  (bind _returnvalue_x_2 (`KismetMathLibrary.BreakVector` (`self.K2_GetActorLocation`)))
  (if (> _returnvalue_x 130.0)
    (`self.K2_SetActorLocation` (`KismetMathLibrary.MakeVector` 130.0 _returnvalue_y _returnvalue_z))
    (elif (< _returnvalue_x -90.0)
      (`self.K2_SetActorLocation` (`KismetMathLibrary.MakeVector` -90.0 _returnvalue_y _returnvalue_z))))
  (bind _returnvalue (`GameplayStatics.GetActorOfClass` "/Game/Volocube/Blueprints/BP_Ball.BP_Ball_C"))
  (bind _returnvalue_x_3 (`KismetMathLibrary.BreakVector` (`self.K2_GetActorLocation` _returnvalue)))
  (bind _returnvalue_2 (- _returnvalue_x_3 _returnvalue_x_2))
  (`KismetSystemLibrary.PrintString` (`KismetStringLibrary.Conv_DoubleToString` _returnvalue_2) true true (struct :`G` 0.66 :`B` 1.0 :`A` 1.0) 0.0)
  (`self.AddMovementInput` (`KismetMathLibrary.MakeVector` (select `bool` (> _returnvalue_2 0.0) :`false` -1.0 :`true` 1.0))))

(fn `UserConstructionScript`
  (`parent.UserConstructionScript`))