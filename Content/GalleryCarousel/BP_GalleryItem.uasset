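; BP_GalleryItem is a single item in a gallery carousel that slides between its neighbors' positions.
; On BeginPlay it caches the pawn and binds to the HUD's Next and Prev dispatchers, retrying until the HUD is valid.
; Each event sets the target to the linked NextItem or PrevItem actor's current location.
; Tick eases the actor toward that target and yaw-billboards its plane toward the pawn's camera.
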(event `self.ReceiveBeginPlay`
  (`|ExecutionSequence`
    (:`then_0`
      (bind _asbp_pawn (cast `/Game/GalleryCarousel/BP_Pawn` (`GameplayStatics.GetPlayerPawn` 0)))
      (set `self.PawnRef` _asbp_pawn)
      (set `self.NextLoc` (`self.K2_GetActorLocation`)))
    (:`then_1`
      (bind _asbp_pc (cast `/Game/GalleryCarousel/BP_PC` (`GameplayStatics.GetPlayerController` 0) :!label _label))
      (bind _hud_ref (`/Game/GalleryCarousel/BP_PC.HUD_ref` _asbp_pc)
        (:`then`
          (add `/Game/GalleryCarousel/WBP_Gallery_Carousel.onNext` _hud_ref (delegate `onNext_Event`))
          (add `/Game/GalleryCarousel/WBP_Gallery_Carousel.onPrev` _hud_ref (delegate `onPrev_Event`)))
        (:`else`
          (`KismetSystemLibrary.Delay` 0.2)
          (goto _label))))))

(event `onNext_Event`
  (set `self.NextLoc` (`self.K2_GetActorLocation` (`self.NextItem`))))

(event `onPrev_Event`
  (set `self.NextLoc` (`self.K2_GetActorLocation` (`self.PrevItem`))))

(event `self.ReceiveTick`
  (params (DeltaSeconds :type "Float (single-precision)"))
  (bind (_returnvalue_roll _returnvalue_pitch _returnvalue_yaw) (`KismetMathLibrary.BreakRotator` (`KismetMathLibrary.FindLookAtRotation` (`SceneComponent.K2_GetComponentLocation` (`/Game/GalleryCarousel/BP_Pawn.Camera` (`self.PawnRef`))) (`SceneComponent.K2_GetComponentLocation` (`self.Plane`)))))
  (`|ExecutionSequence`
    (:`then_0`
      (`SceneComponent.K2_SetWorldRotation` (`self.Plane`) (`KismetMathLibrary.MakeRotator` 90.0 0.0 (+ _returnvalue_yaw 90.0)) false false))
    (:`then_1`
      (`self.K2_SetActorLocation` (`KismetMathLibrary.VInterpTo` (`self.K2_GetActorLocation`) (`self.NextLoc`) DeltaSeconds 5.0)))))

(fn `UserConstructionScript`)