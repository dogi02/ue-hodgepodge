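; BP_MazeWalker is an actor that carves a random-walk path through blocking geometry at BeginPlay, apparently to generate a maze.
; Over a fixed loop, it picks a neighbouring cell along its forward or right axis and line-traces to it.
; On a hit, it teleports the struck component far away, steps in and records the location.
; On a miss, it takes one unchecked random step per recorded location.
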(event `self.ReceiveBeginPlay`
  (for _ (range 101)
    (bind _success (`self.move to cell`))
    (if _success
      (`self.add new location`)
      (else
        (`self.check location`)))))

(fn `add new location`
  (`KismetArrayLibrary.Array_AddUnique` (`self.locations 4 walker`) (`self.K2_GetActorLocation`))
  (return))

(fn `check location`
  (bind _locations_4_walker (`self.locations 4 walker`))
  (for _array_element _locations_4_walker
    (if (`KismetArrayLibrary.Array_Contains` _locations_4_walker _array_element)
      (bind _returnvalue (`self.Sellect Cell`))
      (`self.K2_SetActorLocation` _returnvalue))))

(fn `move to cell`
  (returns (success :type Boolean))
  (bind _returnvalue (`self.Sellect Cell`))
  (bind (_outhit _returnvalue_2) (`KismetSystemLibrary.LineTraceSingle` (`self.K2_GetActorLocation`) _returnvalue "TraceTypeQuery1" false (`|MakeArray` self :!type "Actor Object Reference") "ForDuration" true (struct :`R` 1.0 :`A` 1.0) (struct :`G` 1.0 :`A` 1.0) 60.0))
  (if _returnvalue_2
    (`SceneComponent.K2_SetWorldLocation` (`.HitComponent` (`GameplayStatics.BreakHitResult` _outhit)) (999999.0 0.0 0.0) false false)
    (`self.K2_SetActorLocation` _returnvalue)
    (return true)
    (else
      (return false))))

(fn `Sellect Cell`
  (returns (ReturnValue :type "Vector Structure"))
  (bind _returnvalue (+ (`self.K2_GetActorLocation`) (* (`KismetMathLibrary.SelectVector` (* (`self.GetActorForwardVector`) (`KismetMathLibrary.SelectInt` 1 -1 (`KismetMathLibrary.RandomBool`))) (* (`self.GetActorRightVector`) (`KismetMathLibrary.SelectInt` 1 -1 (`KismetMathLibrary.RandomBool`))) (`KismetMathLibrary.RandomBool`)) 100)))
  (`KismetArrayLibrary.Array_AddUnique` (`self.list of moves`) _returnvalue)
  (return _returnvalue))

(fn `UserConstructionScript`)