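; BP_Maze is a construction-script actor that lays out a full grid of maze-cell walls on a floor plane scaled by Size.
; Walls1 and Walls2 use nested loops to add thin static mesh segments in two perpendicular sets, offset to center on the plane.
; Walls2 swaps the Size axes in its loops, so the grid only lines up when Size is square.
; No path carving, randomization or runtime logic exists.
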(event `self.ReceiveBeginPlay`)

(fn `UserConstructionScript`
  (bind (_size_x _size_y) (`KismetMathLibrary.BreakVector2D` (`self.size`)))
  (`SceneComponent.SetRelativeScale3D` (`self.Plane`) (`KismetMathLibrary.MakeVector` _size_x _size_y 1.0))
  (`self.walls1`)
  (`self.walls2`))

(fn `walls1`
  (bind (_size_x _size_y) (`KismetMathLibrary.BreakVector2D` (`self.size`)))
  (bind (_returnvalue_x _returnvalue_y) (`KismetMathLibrary.BreakVector2D` (/ (`self.size`) (2.0 2.0))))
  (for _index (range (+ (`KismetMathLibrary.FTrunc` _size_x) 1))
    (for _index_2 (range (`KismetMathLibrary.FTrunc` _size_y))
      (bind _returnvalue_x_2 (`KismetMathLibrary.BreakVector` (* _index 99 (`self.GetActorForwardVector`))))
      (bind (_returnvalue_x_3 _returnvalue_y_2) (`KismetMathLibrary.BreakVector` (* _index_2 100 (`self.GetActorRightVector`))))
      (`AddComponent|NODE_AddStaticMeshComponent-0` :`RelativeTransform` (`KismetMathLibrary.MakeTransform` (`KismetMathLibrary.MakeVector` (+ _returnvalue_x_2 (.x (+ (- (0.0 0.0 0.0) (`KismetMathLibrary.MakeVector` (* _returnvalue_x 100.0) (* _returnvalue_y 100.0))) (5.0 50.0 50.0)))) (+ _returnvalue_y_2 (.y (+ (- (0.0 0.0 0.0) (`KismetMathLibrary.MakeVector` (* _returnvalue_x 100.0) (* _returnvalue_y 100.0))) (5.0 50.0 50.0)))) (.z (+ (- (0.0 0.0 0.0) (`KismetMathLibrary.MakeVector` (* _returnvalue_x 100.0) (* _returnvalue_y 100.0))) (5.0 50.0 50.0)))) (struct) (0.1 1.0 1.0))))))

(fn `walls2`
  (bind (_size_x _size_y) (`KismetMathLibrary.BreakVector2D` (`self.size`)))
  (bind (_returnvalue_x _returnvalue_y) (`KismetMathLibrary.BreakVector2D` (/ (`self.size`) (2.0 2.0))))
  (for _index (range (`KismetMathLibrary.FTrunc` _size_y))
    (for _index_2 (range (+ (`KismetMathLibrary.FTrunc` _size_x) 1))
      (bind _returnvalue_x_2 (`KismetMathLibrary.BreakVector` (* _index 100 (`self.GetActorForwardVector`))))
      (bind (_returnvalue_x_3 _returnvalue_y_2) (`KismetMathLibrary.BreakVector` (* _index_2 99 (`self.GetActorRightVector`))))
      (`AddComponent|NODE_AddStaticMeshComponent-1` :`RelativeTransform` (`KismetMathLibrary.MakeTransform` (`KismetMathLibrary.MakeVector` (+ _returnvalue_x_2 (.x (+ (- (0.0 0.0 0.0) (`KismetMathLibrary.MakeVector` (* _returnvalue_x 100.0) (* _returnvalue_y 100.0))) (50.0 5.0 50.0)))) (+ _returnvalue_y_2 (.y (+ (- (0.0 0.0 0.0) (`KismetMathLibrary.MakeVector` (* _returnvalue_x 100.0) (* _returnvalue_y 100.0))) (50.0 5.0 50.0)))) (.z (+ (- (0.0 0.0 0.0) (`KismetMathLibrary.MakeVector` (* _returnvalue_x 100.0) (* _returnvalue_y 100.0))) (50.0 5.0 50.0)))) (struct) (1.0 0.1 1.0))))))