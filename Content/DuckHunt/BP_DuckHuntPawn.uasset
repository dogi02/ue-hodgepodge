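; Player pawn for the Duck Hunt game: a twin-barrel gun aimed by axis input, with a HUD widget created on BeginPlay.
; While left mouse is held, Tick spawns projectiles from two scene components with random recoil, using a Delay-reset flag to limit fire rate.
; Each volley adds heat; reaching the maximum jams the gun temporarily and notifies the UI.
; Releasing the button starts a looping timer that cools it.
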(event `self.ReceiveBeginPlay`
  (bind _returnvalue (`|CreateWidget` "/Game/DuckHunt/WBP_DuckHuntUI.WBP_DuckHuntUI_C"))
  (bind _output_get (set `self.DuckHuntUI` _returnvalue))
  (`UserWidget.AddToViewport` _output_get 0)
  (`WidgetBlueprintLibrary.SetInputMode_GameOnly` (`GameplayStatics.GetPlayerController` 0)))

(event `self.ReceiveTick`
  (params (DeltaSeconds :type "Float (single-precision)"))
  (bind (_returnvalue_location _returnvalue_rotation) (`KismetMathLibrary.BreakTransform` (`SceneComponent.K2_GetComponentToWorld` (`self.Scene1`))))
  (bind (_returnvalue_location_2 _returnvalue_rotation_2) (`KismetMathLibrary.BreakTransform` (`SceneComponent.K2_GetComponentToWorld` (`self.Scene`))))
  (`|ExecutionSequence`
    (:`then_0`
      (`self.AddControllerYawInput` (* (`self.GetInputAxisKeyValue`) (`self.RotationSpeedMultiplier`)))
      (`self.AddControllerPitchInput` (* (`self.GetInputAxisKeyValue`) (`self.RotationSpeedMultiplier`) -1.0)))
    (:`then_1`
      (if (and (`self.isFiring`) (not (`self.isReloading`)) (not (`self.isJammed`)))
        (`|SpawnActorFromClass` "/Game/DuckHunt/BP_Projectile.BP_Projectile_C" (`KismetMathLibrary.MakeTransform` _returnvalue_location _returnvalue_rotation) "Undefined" "MultiplyWithRoot" null null)
        (`|SpawnActorFromClass` "/Game/DuckHunt/BP_Projectile.BP_Projectile_C" (`KismetMathLibrary.MakeTransform` _returnvalue_location_2 _returnvalue_rotation_2) "Undefined" "MultiplyWithRoot" null null)
        (`self.AddControllerPitchInput` (`KismetMathLibrary.RandomFloatInRange` -0.3 -0.1))
        (`self.AddControllerYawInput` (`KismetMathLibrary.SelectFloat` -0.1 0.1 (`KismetMathLibrary.RandomBool`)))
        (`/Engine/EditorBlueprintResources/StandardMacros.IncrementInt` (`self.HeatCounter`)
          (:`  `
            (set `self.isReloading` true)
            (`KismetSystemLibrary.Delay` 0.075)
            (set `self.isReloading` false)))))
    (:`then_2`
      (if (>= (`self.HeatCounter`) (`self.MaxHeat`))
        (set `self.isJammed` true)
        (`/Game/DuckHunt/WBP_DuckHuntUI.Jammed` (`self.DuckHuntUI`) true)
        (`KismetSystemLibrary.Delay` 3.0)
        (`/Game/DuckHunt/WBP_DuckHuntUI.Jammed` (`self.DuckHuntUI`) false)
        (set `self.isJammed` false)
        (set `self.HeatCounter` 0)))))

(event `Key|LeftMouseButton`
  (params (Key :type "Key Structure"))
  (:`Pressed`
    (set `self.isFiring` true)
    (`KismetSystemLibrary.K2_ClearAndInvalidateTimerHandle` (stale _returnvalue) :!label _label))
  (:`Released`
    (set `self.isFiring` false)
    (bind _returnvalue (`KismetSystemLibrary.K2_SetTimerDelegate` (delegate `AutoCooling`) 0.05 true))))

(event `AutoCooling`
  (bind _heatcounter (`self.HeatCounter`))
  (if (not (`self.isJammed`))
    (if (<= _heatcounter 0)
      (goto _label)
      (else
        (`/Engine/EditorBlueprintResources/StandardMacros.DecrementInt` _heatcounter)))))

(fn `UserConstructionScript`)