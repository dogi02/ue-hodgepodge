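; BP_MainPC is a player controller that manages input modes and opens the pause menu on Escape.
; It creates the pause widget at BeginPlay, then on Escape adds it to the viewport, saves the previous input mode, switches to UI-only and centers the mouse.
; SetAdvancedInputMode wraps the engine input-mode calls, validating the focus widget and tracking mode and cursor visibility.
; Menu opened and closed events are empty hooks.
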(event `self.ReceiveBeginPlay`
  (`self.AddUI`)
  (`self.SetAdvancedInputMode` "NewEnumerator0" null true false))

(event `Key|Escape`
  (params (Key :type "Key Structure"))
  (:`Pressed`
    (`self.TryToAddPauseMenu`)))

(event `OnPauseMenuOpened`)

(event `OnPauseMenuClosed`)

(fn `AddUI`
  (bind _returnvalue (`|CreateWidget` "/Game/MainBlueprints/UMG/MainMenu/WBP_PauseMenu.WBP_PauseMenu_C" null self))
  (set `self.PauseMenuUI` _returnvalue))

(fn `SetAdvancedInputMode`
  (params (InputMode :type "/Game/MainBlueprints/Enums/EInputMode Enum" :default "NewEnumerator0") (WidgetToFocus :type "Widget Object Reference") (FlushInput :type Boolean :default true) (ShowCursor :type Boolean :default true))
  (returns (Succes :type Boolean))
  (switch `/Game/MainBlueprints/Enums/EInputMode` InputMode
    (:`NewEnumerator0`
      (`WidgetBlueprintLibrary.SetInputMode_GameOnly` self (`local.FlushInput`)))
    (:`NewEnumerator1`
      (`/Engine/EditorBlueprintResources/StandardMacros.IsValid` (`local.WidgetToFocus`)
        (:`Is Valid`
          (`WidgetBlueprintLibrary.SetInputMode_UIOnlyEx` self (`local.WidgetToFocus`) "DoNotLock" (`local.FlushInput`)))
        (:`Is Not Valid`
          (return false))))
    (:`NewEnumerator2`
      (`/Engine/EditorBlueprintResources/StandardMacros.IsValid` (`local.WidgetToFocus`)
        (:`Is Valid`
          (`WidgetBlueprintLibrary.SetInputMode_GameAndUIEx` self (`local.WidgetToFocus`) "DoNotLock" true (`local.FlushInput`)))
        (:`Is Not Valid`
          (return false)))))
  (set `self.CurrentInputMode` (`local.InputMode`))
  (set `self.bShowMouseCursor` (`local.ShowCursor`))
  (return true))

(fn `TryToAddPauseMenu`
  (bind (_sizex _sizey) (`self.GetViewportSize`))
  (bind _pausemenuui (`self.PauseMenuUI`))
  (bind _pausemenuui_2 (`self.PauseMenuUI`)
    (:`then`
      (if (not (`Widget.IsVisible` _pausemenuui_2))
        (`UserWidget.AddToViewport` _pausemenuui 0)
        (set `self.LastInputMode` (`self.CurrentInputMode`))
        (`self.SetAdvancedInputMode` "NewEnumerator1" _pausemenuui)
        (`self.SetMouseLocation` (/ _sizex 2) (/ _sizey 2))
        (`self.OnPauseMenuOpened`)))
    (:`else`)))

(fn `UserConstructionScript`)